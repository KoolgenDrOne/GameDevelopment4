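; Elevator actor that rises a fixed height and returns to its start when the player interacts with it.
; BeginPlay stores the start and target Z, then binds to the OnInteract dispatcher on BP_TestController.
; Player overlap with the box enables interaction while idle; leaving never clears it.
; Interacting locks input and plays two chained timelines that lerp Z up and straight back down, then re-enables interaction.
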(event `self.ReceiveBeginPlay`
  (bind (_returnvalue_x _returnvalue_y _returnvalue_z) (`KismetMathLibrary.BreakVector` (`self.K2_GetActorLocation`)))
  (bind _output_get (set `self.ElevatorInitialLocation` _returnvalue_z :!pinned true)) ; Taking the initial location of this actor and storing it
  (set `self.ElevatorStepOffset` (+ _output_get 1000.0) :!pinned true) ; Setting this as final location
  (bind _asbp_test_controller (cast `/Game/GD4/BP/BP_TestController` (`GameplayStatics.GetPlayerController` 0))) ; Converting general player controller class to Out specific player controller class
  (add `/Game/GD4/BP/BP_TestController.OnInteract` _asbp_test_controller (delegate `OnInteract_Event`) :!pinned true) ; Suscribing to and dispatcher called on Interact in our Custom Player controller\nThis is pointer to a function which gets executed when certain(interact) input is given \nin Player Controller\nThis also gives a function Callback with matching function signature
)

(event `OnInteract_Event`
  (bind (_returnvalue_x _returnvalue_y) (`KismetMathLibrary.BreakVector` (`self.K2_GetActorLocation`)))
  (bind (_returnvalue_x_2 _returnvalue_y_2) (`KismetMathLibrary.BreakVector` (`self.K2_GetActorLocation`)))
  (if (`self.bCanInteract`) :!pinned true
    (set `self.bCanInteract` false)
    (set `self.bIsElevatorMoving` true)
    (bind (_direction _out) (`Timeline|ElevatorMovement` :!pinned true :!via `PlayFromStart`) ; Timeline is special node which fires every frame for specified duration\nWe are using it to lerp between a float value that goes from 0 to 1 over duration of 5 sec\n(Double click to open this node)
      (:`Update`
        (`self.K2_SetActorLocation` (`KismetMathLibrary.MakeVector` _returnvalue_x_2 _returnvalue_y_2 (`KismetMathLibrary.Lerp` (`self.ElevatorInitialLocation`) (`self.ElevatorStepOffset`) _out)) :!pinned true) ; Changing the actor loation smoothly over duration of 5 second\nOnly changing Z axis as elevator goes UP and DOWN\nX and Y can stay as they are
      )
      (:`Finished`
        (bind (_direction_2 _out_2) (`Timeline|Timeline` :!pinned true :!via `PlayFromStart`) ; Same as above timeline but reverse
          (:`Update`
            (`self.K2_SetActorLocation` (`KismetMathLibrary.MakeVector` _returnvalue_x _returnvalue_y (`KismetMathLibrary.Lerp` (`self.ElevatorStepOffset`) (`self.ElevatorInitialLocation`) _out_2))))
          (:`Finished`
            (set `self.bIsElevatorMoving` false)
            (set `self.bCanInteract` true)))))))

(event `self.Box.OnComponentBeginOverlap`
  (params (OverlappedComponent :type "PrimitiveComponent Object Reference") (OtherActor :type "Actor Object Reference") (OtherComp :type "PrimitiveComponent Object Reference") (OtherBodyIndex :type Integer) (bFromSweep :type Boolean) (SweepResult :type "HitResult Structure (by ref)"))
  (if (and (== OtherActor (`GameplayStatics.GetPlayerCharacter` 0)) (not (`self.bIsElevatorMoving`))) :!pinned true
    (set `self.bCanInteract` true) ; We can interact with is actor
  ))

(fn `UserConstructionScript`)