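; BP_FirstActor is a demo actor that shows when basic Actor events fire by printing colored debug messages to the screen.
; BeginPlay prints once on spawn, and Tick prints every frame.
; When the player character begins overlapping its Box component, it increments OverlapCounter and prints the overlapping actor's name with the running count.
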(event `self.ReceiveBeginPlay`
  (`KismetSystemLibrary.PrintString` "Begin Play Fired" true true (struct :`R` 1.0 :`B` 0.019891 :`A` 1.0) 25.0))

(event `self.ReceiveTick`
  (params (DeltaSeconds :type "Float (single-precision)"))
  (`KismetSystemLibrary.PrintString` "Tick Firing" true true (struct :`R` 0.07124 :`G` 1.0 :`A` 1.0) 0.0))

(event `self.Box.OnComponentBeginOverlap`
  (params (OverlappedComponent :type "PrimitiveComponent Object Reference") (OtherActor :type "Actor Object Reference") (OtherComp :type "PrimitiveComponent Object Reference") (OtherBodyIndex :type Integer) (bFromSweep :type Boolean) (SweepResult :type "HitResult Structure (by ref)"))
  (if (== OtherActor (`GameplayStatics.GetPlayerCharacter` 0))
    (bind _output_get (set `self.OverlapCounter` (+ (`self.OverlapCounter`) 1)))
    (`KismetSystemLibrary.PrintString` (`KismetStringLibrary.Concat_StrStr` (`KismetSystemLibrary.GetDisplayName` OtherActor) " Has Overlapped this actor :" (`KismetStringLibrary.Conv_IntToString` _output_get) " Times") true true (struct :`R` 0.051206 :`B` 1.0 :`A` 1.0) 25.0)))

(fn `UserConstructionScript`)